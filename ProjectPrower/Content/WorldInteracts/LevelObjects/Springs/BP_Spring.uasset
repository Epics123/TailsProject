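; BP_Spring is a world spring that launches characters along a velocity set by its rotation and LaunchPower.
; Launch snaps the character to the launch point, zeroes falling braking, applies the velocity, optionally plays an air montage, and triggers spring sound and animation.
; Characters turn toward the launch direction unless the spring's rotation is near zero.
; The construction script rebuilds a spline from the predicted projectile path to show the trajectory.
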(event `self.Launch`
  (params (Character :type "ProjectProwerCharacter Object Reference"))
  (`parent.Launch` Character)
  (`self.K2_SetActorLocation` Character (`SceneComponent.K2_GetComponentLocation` (`self.SpringLaunchPoint`)) false true) ; Ensure we're always launched from the center of the spring
  (if (`self.PlayAirAnimation`)
    (`Character.PlayAnimMontage` Character (`self.LaunchMontage`) 1.0 "None"))
  (set `CharacterMovementComponent.BrakingDecelerationFalling` 0.0 (`ProjectProwerCharacter.GetProwerMovementComponent` Character))
  (`Character.LaunchCharacter` Character (`self.GetLaunchVelocity`) true true)
  (`self.RotateCharacterToVelocity` Character)
  (`GameplayStatics.PlaySoundAtLocation` "/Game/WorldInteracts/LevelObjects/Springs/SFX/SE_Spring.SE_Spring" (`self.K2_GetActorLocation`) (struct) 1.0 1.0 0.0 "/Game/Audio/SA_Common.SA_Common" null null null)
  (`SkeletalMeshComponent.PlayAnimation` (`self.SpringMesh`) "/Game/WorldInteracts/LevelObjects/Springs/AS_Spring.AS_Spring" false))

(event `RotateCharacterToVelocity`
  (params (Character :type "ProjectProwerCharacter Object Reference"))
  (bind _returnvalue (`self.K2_GetActorLocation` Character))
  (if (not (== (`self.K2_GetActorRotation`) (struct) :`ErrorTolerance` 0.001))
    (`self.K2_SetActorRotation` Character (`KismetMathLibrary.FindLookAtRotation` _returnvalue (+ _returnvalue (`self.GetLaunchVelocity`))) false)))

(fn `GetLaunchVelocity`
  (returns (Velocity :type "Vector Structure"))
  (return (`KismetMathLibrary.GreaterGreater_VectorRotator` (+ (`self.GetActorForwardVector`) (`KismetMathLibrary.MakeVector` 0.0 0.0 (`self.LaunchPower`))) (`self.K2_GetActorRotation`))))

(fn `UserConstructionScript`
  (`SplineComponent.ClearSplinePoints` (`self.SpringTrajectoryPath`) true)
  (bind _predictresult (`GameplayStatics.Blueprint_PredictProjectilePath_Advanced` (make `PredictProjectilePathParams` (`self.K2_GetActorLocation`) (`self.GetLaunchVelocity`))))
  (for _array_element (break `PredictProjectilePathResult` _predictresult)
    (`SplineComponent.AddSplinePoint` (`self.SpringTrajectoryPath`) (`.Location` (break `PredictProjectilePathPointData` _array_element)) "World" true)))