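; BP_DashRamp is a level object that launches the character along an arc set by launch and vertical power, rotated to the ramp.
; Launch overrides velocity, zeroes falling braking, faces the character along the trajectory, and plays a montage and jumpboard sound.
; Ramp collision switches off at launch and returns when a ProjectProwerCharacter ends overlap.
; The construction script previews the predicted projectile path as a spline from a debug launch point.
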(event `self.Launch`
  (params (Character :type "ProjectProwerCharacter Object Reference"))
  (`parent.Launch` Character)
  (set `CharacterMovementComponent.BrakingDecelerationFalling` 0.0 (`ProjectProwerCharacter.GetProwerMovementComponent` Character))
  (`PrimitiveComponent.SetCollisionEnabled` (`self.DashRamp`) "NoCollision")
  (`Character.PlayAnimMontage` Character (`self.LaunchMontage`) 0.5 "Default")
  (`Character.LaunchCharacter` Character (`self.GetLaunchVelocity`) true true)
  (`self.RotateCharacterToVelocity` Character)
  (`GameplayStatics.PlaySoundAtLocation` "/Game/WorldInteracts/LevelObjects/DashRamp/SFX/SE_Jumpboard.SE_Jumpboard" (`self.K2_GetActorLocation`) (struct) 1.0 1.0 0.0 "/Game/Audio/SA_Common.SA_Common" null null null))

(event `self.ReceiveActorEndOverlap`
  (params (OtherActor :type "Actor Object Reference"))
  (cast `ProjectProwerCharacter` OtherActor)
  (`PrimitiveComponent.SetCollisionEnabled` (`self.DashRamp`) "QueryAndPhysics"))

(event `RotateCharacterToVelocity`
  (params (Character :type "ProjectProwerCharacter Object Reference"))
  (bind _returnvalue (`self.K2_GetActorLocation` Character))
  (`self.K2_SetActorRotation` Character (`KismetMathLibrary.FindLookAtRotation` _returnvalue (+ _returnvalue (`self.GetLaunchVelocity`))) false))

(fn `GetLaunchVelocity`
  (returns (Velocity :type "Vector Structure"))
  (return (`KismetMathLibrary.GreaterGreater_VectorRotator` (+ (`self.GetActorForwardVector`) (`KismetMathLibrary.MakeVector` (`self.LaunchPower`) 0.0 (`self.VerticalPower`))) (`self.K2_GetActorRotation`))))

(fn `UserConstructionScript`
  (`SplineComponent.ClearSplinePoints` (`self.LaunchTrajectoryPath`) true)
  (bind _predictresult (`GameplayStatics.Blueprint_PredictProjectilePath_Advanced` (make `PredictProjectilePathParams` (`SceneComponent.K2_GetComponentLocation` (`self.DebugLaunchPoint`)) (`self.GetLaunchVelocity`))))
  (for _array_element (break `PredictProjectilePathResult` _predictresult)
    (`SplineComponent.AddSplinePoint` (`self.LaunchTrajectoryPath`) (`.Location` (break `PredictProjectilePathPointData` _array_element)) "World" true)))