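; Base Blueprint for launch objects that prepare an overlapping player character for launch; no launch velocity is applied here.
; Box overlap resets jumpball and flight state, then optionally blocks flight and movement input, with timers for each lock.
; Unlock events fire dispatchers and clear their bindings; for BP_Tails, a valid launch montage also hooks landing, and ClearMontage stops it.
; The construction script scales an arrow's length by LaunchPower as a preview.
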(event `UnlockFlight`
  (`self.OnFlightUnlocked`)
  (clear `self.OnFlightUnlocked`))

(event `UnlockMoveInput`
  (`self.OnMovementUnlocked`)
  (clear `self.OnMovementUnlocked`))

(event `LockFlight`
  (if (`self.bLockFlight`)
    (`ProjectProwerCharacter.SetFlightBlocked` (`self.Player`) true)
    (`KismetSystemLibrary.K2_SetTimerDelegate` (`|CreateDelegate` :!event `UnlockFlight`) (`self.FlightLockDuration`))))

(event `SetupBindings`
  (params (Character :type "ProjectProwerCharacter Object Reference"))
  (bind _asbp_tails (cast `/Game/Characters/Tails/BP_Tails` Character))
  (add `self.OnFlightUnlocked` (`|CreateDelegate` _asbp_tails :!event `UnblockFlight`))
  (add `self.OnMovementUnlocked` (`|CreateDelegate` _asbp_tails :!event `UnblockMovement`))
  (`/Engine/EditorBlueprintResources/StandardMacros.IsValid` (`self.LaunchMontage`)
    (:`Is Valid`
      (add `/Game/Characters/Tails/BP_Tails.OnCharacterLanded` _asbp_tails (`|CreateDelegate` :!event `ClearMontage`)))))

(event `LockMovement`
  (if (`self.bLockMovement`)
    (`ProjectProwerCharacter.SetMoveInputBlocked` (`self.Player`) true)
    (`KismetSystemLibrary.K2_SetTimerDelegate` (`|CreateDelegate` :!event `UnlockMoveInput`) (`self.MovementLockDuration`))))

(event `self.Launch`
  (params (Character :type "ProjectProwerCharacter Object Reference"))
  (`ProjectProwerCharacter.ToggleJumpballMesh` Character false)
  (`ProjectProwerCharacter.ResetFlightState` Character)
  (`self.LockFlight`)
  (`self.LockMovement`)
  (`self.SetupBindings` Character))

(event `self.Box.OnComponentBeginOverlap`
  (params (OverlappedComponent :type "PrimitiveComponent Object Reference") (OtherActor :type "Actor Object Reference") (OtherComp :type "PrimitiveComponent Object Reference") (OtherBodyIndex :type Integer) (bFromSweep :type Boolean) (SweepResult :type "HitResult Structure (by ref)"))
  (bind _asproject_prower_character (cast `ProjectProwerCharacter` OtherActor))
  (bind _output_get (set `self.Player` _asproject_prower_character))
  (`self.Launch` _output_get))

(event `ClearMontage`
  (`/Engine/EditorBlueprintResources/StandardMacros.IsValid` (`self.LaunchMontage`)
    (:`Is Valid`
      (`Character.StopAnimMontage` (`self.Player`) (`self.LaunchMontage`))
      (bind _asbp_tails (cast `/Game/Characters/Tails/BP_Tails` (`self.Player`)))
      (remove `/Game/Characters/Tails/BP_Tails.OnCharacterLanded` _asbp_tails (`|CreateDelegate` :!event `ClearMontage`)))
    (:`Is Not Valid`
      _))
  (set `self.Player` null))

(fn `UserConstructionScript`
  (`SceneComponent.SetWorldScale3D` (`self.Arrow`) (`KismetMathLibrary.MakeVector` (/ (/ (`self.LaunchPower`) 100.0) 2.0) 1.0 1.0)))