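; BP_CMT_FixedTransform is a world-placed camera actor, a child Blueprint that supplies a fixed-transform camera mode to a camera component.
; On PushCameraMode it constructs the configured CameraMode class and continues only if the instance is a FixedTransformCameraMode.
; It composes CameraTransform with the actor's transform to set the target in world space, then pushes that instance onto the CameraComponent.
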(event `self.ReceiveBeginPlay`
  (`parent.ReceiveBeginPlay`))

(event `self.PushCameraMode`
  (bind _returnvalue (`|GenericCreateObject` (`self.CameraMode`)))
  (bind _asfixed_transform_camera_mode (cast `FixedTransformCameraMode` _returnvalue))
  (set `FixedTransformCameraMode.TargetTransform` (`KismetMathLibrary.ComposeTransforms` (`self.CameraTransform`) (`self.GetTransform`)) _asfixed_transform_camera_mode)
  (`ProwerCameraComponent.PushCameraModeInstance` (`self.CameraComponent`) _asfixed_transform_camera_mode))

(fn `UserConstructionScript`
  (`parent.UserConstructionScript`))