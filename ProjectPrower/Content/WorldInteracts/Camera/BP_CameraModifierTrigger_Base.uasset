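; Base trigger volume that switches the camera mode of an actor entering its box.
; On begin overlap it finds and stores that actor's camera component, then pushes the configured CameraMode class onto it.
; On end overlap it pushes BP_CameraMode_Default onto the stored component rather than removing the mode, without checking which actor left.
; The construction script labels a text render with the chosen mode's name.
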(event `self.ReceiveBeginPlay`)

(event `self.Box.OnComponentBeginOverlap`
  (params (OverlappedComponent :type "PrimitiveComponent Object Reference") (OtherActor :type "Actor Object Reference") (OtherComp :type "PrimitiveComponent Object Reference") (OtherBodyIndex :type Integer) (bFromSweep :type Boolean) (SweepResult :type "HitResult Structure (by ref)"))
  (set `self.CameraComponent` (`ProwerCameraComponent.FindCameraComponent` OtherActor))
  (`/Engine/EditorBlueprintResources/StandardMacros.IsValid` (`self.CameraComponent`)
    (:`Is Valid`
      (`self.PushCameraMode`))))

(event `self.Box.OnComponentEndOverlap`
  (params (OverlappedComponent :type "PrimitiveComponent Object Reference") (OtherActor :type "Actor Object Reference") (OtherComp :type "PrimitiveComponent Object Reference") (OtherBodyIndex :type Integer))
  (`/Engine/EditorBlueprintResources/StandardMacros.IsValid` (`self.CameraComponent`)
    (:`Is Valid`
      (`self.PopCameraMode`))))

(event `PushCameraMode`
  (bind _cameramode (`self.CameraMode`))
  (if (`KismetSystemLibrary.IsValidClass` _cameramode)
    (`ProwerCameraComponent.PushCameraMode` (`self.CameraComponent`) _cameramode)))

(event `PopCameraMode`
  (`ProwerCameraComponent.PushCameraMode` (`self.CameraComponent`) "/Game/Data/CameraModes/BP_CameraMode_Default.BP_CameraMode_Default_C"))

(fn `UserConstructionScript`
  (if (`KismetSystemLibrary.IsValidClass` (`self.CameraMode`))
    (`TextRenderComponent.K2_SetText` (`self.TextRender`) (`|FormatText` "Camera Mode: {Mode}" (`KismetSystemLibrary.GetClassDisplayName` (`self.CameraMode`))))))