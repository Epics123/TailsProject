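; BP_Tails is the Blueprint for the Tails character, and its only active logic is a per-frame debug visualisation of movement and facing.
; On Tick it draws colour-coded arrows from the actor's location for the normalised horizontal velocity, forward vector and right vector.
; The velocity arrow flattens Z, so travel direction can be compared against the actor's orientation.
; BeginPlay, overlap and construction logic are empty.
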(event `self.ReceiveTick`
  (params (DeltaSeconds :type "Float (single-precision)"))
  (bind _returnvalue (`self.K2_GetActorLocation`))
  (bind _returnvalue_2 (`self.K2_GetActorLocation`))
  (bind _returnvalue_3 (`self.K2_GetActorLocation`))
  (`KismetSystemLibrary.DrawDebugArrow` _returnvalue_3 (+ _returnvalue_3 (* (`KismetMathLibrary.Normal` (`KismetMathLibrary.MakeVector` (.x (`MovementComponent.Velocity` (`self.CharacterMovement`))) (.y (`MovementComponent.Velocity` (`self.CharacterMovement`))))) 50.0)) 1.0 (struct :`R` 0.950309 :`G` 0.054318 :`B` 1.0 :`A` 1.0) 0.0 1.0)
  (`KismetSystemLibrary.DrawDebugArrow` _returnvalue (+ _returnvalue (* (`self.GetActorForwardVector`) 50.0)) 1.0 (struct :`R` 1.0 :`G` 0.033106 :`A` 1.0) 0.0 1.0)
  (`KismetSystemLibrary.DrawDebugArrow` _returnvalue_2 (+ _returnvalue_2 (* (`self.GetActorRightVector`) 50.0)) 1.0 (struct :`R` 0.095426 :`G` 1.0 :`A` 1.0) 0.0 1.0))

(fn `UserConstructionScript`)